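; Game instance that holds the global, effects, voice and music volume settings and persists them through BP_Default_SaveGame.
; On Init it restores the volumes from the "default" slot if that save exists.
; SetSpecificVolume updates one channel by audio type and immediately saves all four, reusing or creating the save object.
; Saving targets the SaveSlotName variable, while loading uses the hardcoded "default" slot name.
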(event `self.ReceiveInit`
  (bind _returnvalue (`GameplayStatics.DoesSaveGameExist` "default"))
  (if _returnvalue
    (`self.GetVolumeInfoFromSave`)))

(fn `GetVolumeInfoFromSave`
  (bind _returnvalue (`GameplayStatics.LoadGameFromSlot` "default"))
  (bind _asbp_default_save_game (cast `/Game/Blueprints/Core/BP_Default_SaveGame` _returnvalue))
  (set `self.Volume_Global` (`/Game/Blueprints/Core/BP_Default_SaveGame.Volume_Global` _asbp_default_save_game))
  (set `self.Volume_Effects` (`/Game/Blueprints/Core/BP_Default_SaveGame.Volume_Effects` _asbp_default_save_game))
  (set `self.Volume_Voice` (`/Game/Blueprints/Core/BP_Default_SaveGame.Volume_Voice` _asbp_default_save_game))
  (set `self.Volume_Music` (`/Game/Blueprints/Core/BP_Default_SaveGame.Volume_Music` _asbp_default_save_game)))

(fn `SaveVolumeInfo`
  (locals (SaveSlotName :type String :default "default"))
  (bind _saveslotname (`local.SaveSlotName`))
  (bind _returnvalue (`GameplayStatics.DoesSaveGameExist` _saveslotname))
  (if _returnvalue
    (bind _returnvalue_2 (`GameplayStatics.LoadGameFromSlot` _saveslotname))
    (bind _asbp_default_save_game (cast `/Game/Blueprints/Core/BP_Default_SaveGame` _returnvalue_2))
    (`self.SetSaveVolumeInfo` _asbp_default_save_game (`local.SaveSlotName`))
    (else
      (bind _returnvalue_3 (`GameplayStatics.CreateSaveGameObject` "/Game/Blueprints/Core/BP_Default_SaveGame.BP_Default_SaveGame_C"))
      (`self.SetSaveVolumeInfo` _returnvalue_3 (`local.SaveSlotName`)))))

(fn `SetSaveVolumeInfo`
  (params (SaveGame :type "/Game/Blueprints/Core/BP_Default_SaveGame Object Reference") (SlotName :type String))
  (set `/Game/Blueprints/Core/BP_Default_SaveGame.Volume_Global` (`self.Volume_Global`) SaveGame)
  (set `/Game/Blueprints/Core/BP_Default_SaveGame.Volume_Effects` (`self.Volume_Effects`) SaveGame)
  (set `/Game/Blueprints/Core/BP_Default_SaveGame.Volume_Voice` (`self.Volume_Voice`) SaveGame)
  (set `/Game/Blueprints/Core/BP_Default_SaveGame.Volume_Music` (`self.Volume_Music`) SaveGame)
  (`GameplayStatics.SaveGameToSlot` SaveGame SlotName))

(fn `SetSpecificVolume`
  (params (AudioType :type "/DefaultUI/Enums/EAudioTypes Enum" :default "NewEnumerator0") (NewVolume :type "Float (double-precision)"))
  (switch `/DefaultUI/Enums/EAudioTypes` AudioType
    (:`NewEnumerator0`
      (set `self.Volume_Global` NewVolume))
    (:`NewEnumerator1`
      (set `self.Volume_Effects` NewVolume))
    (:`NewEnumerator2`
      (set `self.Volume_Voice` NewVolume))
    (:`NewEnumerator3`
      (set `self.Volume_Music` NewVolume)))
  (`self.SaveVolumeInfo`))