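; BP_BarFightGenerator registers itself with the game instance as the bar fight generator.
; On BeginPlay it also caches the player controller's HUD.
; Unconnected test chains, which never run, would generate enemy info, show it in a stat display widget on the HUD with UI-only input, and remove that widget after a delay.
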(event `self.ReceiveBeginPlay`
  (bind _asbp_default_game_instance (cast `/Game/Blueprints/Core/BP_Default_GameInstance` (`GameplayStatics.GetGameInstance`)))
  (bind _output_get (set `self.GameInstanceRef` _asbp_default_game_instance))
  (set `/Game/Blueprints/Core/BP_Default_GameInstance.BarFightGenerator` self _output_get)
  (bind _asbp_player_controller (cast `/Game/Blueprints/Player/BP_PlayerController` (`GameplayStatics.GetPlayerController` 0)))
  (set `self.PlayerHUD` (`/Game/Blueprints/Player/BP_PlayerController.CreatedHUD` _asbp_player_controller)))

(fn `UserConstructionScript`)