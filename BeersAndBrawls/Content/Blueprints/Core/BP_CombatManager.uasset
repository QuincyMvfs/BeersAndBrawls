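; Combat manager that registers itself on the game instance and supplies randomized combat patterns to the player's combat component.
; BeginPlay waits briefly, then caches the game instance and player references.
; RegeneratePattern, after a delay, draws combat and counter patterns from random abilities of the selected weapon, but applies only the combat pattern.
; EngageCombat is empty, and binding regeneration to pattern completion sits in unconnected logic.
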(event `self.ReceiveBeginPlay`
  (`KismetSystemLibrary.Delay` 0.2)
  (bind _asbp_default_game_instance (cast `/Game/Blueprints/Core/BP_Default_GameInstance` (`GameplayStatics.GetGameInstance`)))
  (bind _output_get (set `self.GameInstanceRef` _asbp_default_game_instance))
  (set `/Game/Blueprints/Core/BP_Default_GameInstance.CombatManager` self _output_get)
  (bind _asbp_player (cast `/Game/Blueprints/Player/BP_Player` (`GameplayStatics.GetPlayerPawn` 0)))
  (set `self.PlayerRef` _asbp_player))

(event `EngageCombat`
  (params (EnemyToEngage :type "EnemyInfo Object Reference")))

(event `RegeneratePattern`
  (bind (_randomcombatpattern _randomcounterpattern) (`self.GetRandomPattern` (`self.PlayerRef`)))
  (`KismetSystemLibrary.Delay` 1.0)
  (set `self.GeneratedCombatPattern` _randomcombatpattern)
  (set `self.GeneratedCounterPattern` _randomcounterpattern)
  (`CombatComponent.SetCombatPattern` (`BeersAndBrawlsCharacter.CombatComponent` (`self.PlayerRef`)) (`self.GeneratedCombatPattern`)))

(fn `GetRandomPattern`
  (params (Player :type "BeersAndBrawlsCharacter Object Reference"))
  (returns (RandomCombatPattern :type "CombatPatterns Structure") (RandomCounterPattern :type "CombatPatterns Structure"))
  (bind _m_itempatterns (`AbilityInfo.M_ItemPatterns` (`KismetArrayLibrary.Array_Random` (`Item.Abilities` (`InventoryComponent.M_SelectedWeapon` (`BeersAndBrawlsCharacter.InventoryComponent` Player))))))
  (return (`KismetArrayLibrary.Array_Random` (`AbilityPattern.CombatPatterns` _m_itempatterns)) (`KismetArrayLibrary.Array_Random` (`AbilityPattern.CounterPatterns` _m_itempatterns))))

(fn `UserConstructionScript`)